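; BP_Car is a player-driven hover car that moves on keyboard or controller axis input.
; Tick traces down from the Cylinder and applies a hover force that scales with ground proximity, clamping top speed and turn rate only while the trace hits.
; InputY builds or brakes Speed for a local actor offset, and InputX builds or decays RotationSpeed to yaw the Cylinder.
; Negative Speed has no cap and snaps to zero when throttle is released.
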(event `self.ReceiveTick`
  (params (DeltaSeconds :type "Float (single-precision)"))
  (bind _returnvalue (`SceneComponent.K2_GetComponentLocation` (`self.Cylinder`)))
  ;[1 1 1] Hover
  (bind (_outhit _returnvalue_2) (`KismetSystemLibrary.LineTraceSingle` :`Start` _returnvalue :`End` (+ _returnvalue (`KismetMathLibrary.MakeVector` 0.0 0.0 (* (`self.HoverTraceLength`) -1.0))) :`TraceChannel` "TraceTypeQuery1" :`DrawDebugType` "ForOneFrame"))
  (if _returnvalue_2
    (`PrimitiveComponent.AddForce` (`self.Cylinder`) (* (`self.HoverForce`) (- 1.0 (/ (`KismetMathLibrary.VSize` (- (`.Location` (`GameplayStatics.BreakHitResult` _outhit)) (`SceneComponent.K2_GetComponentLocation` (`self.Cylinder`)))) (`self.HoverTraceLength`)))) "None" false)
    ;[1 1 1] Speed and rotation Cap
    (if (> (`self.Speed`) (`self.SpeedCap`))
      (set `self.Speed` (`self.SpeedCap`)))
    (if (> (`self.RotationSpeed`) (`self.RotationCap`))
      (set `self.RotationSpeed` (`self.RotationCap`)))
    (if (< (`self.RotationSpeed`) (* (`self.RotationCap`) -1.0))
      (set `self.RotationSpeed` (* (`self.RotationCap`) -1.0)))))

(event `InputAxis|InputY`
  (params (AxisValue :type "Float (single-precision)"))
  ;[1 1 1] Forward and backward movement
  (if (`KismetMathLibrary.NearlyEqual_FloatFloat` AxisValue 0.0 0.0001)
    (bind _output_get (set `self.Speed` (- (`self.Speed`) (* (`GameplayStatics.GetWorldDeltaSeconds`) (`self.Breaks`)))))
    (if (< _output_get 0.0)
      (set `self.Speed` 0.0))
    (else
      (set `self.Speed` (+ (`self.Speed`) (* AxisValue (`GameplayStatics.GetWorldDeltaSeconds`) (`self.Acceleration`))))))
  (`self.K2_AddActorLocalOffset` (`KismetMathLibrary.MakeVector` (`self.Speed`))))

(event `InputAxis|InputX`
  (params (AxisValue :type "Float (single-precision)"))
  ;[1 1 1] Rotation
  (if (`KismetMathLibrary.NearlyEqual_FloatFloat` AxisValue 0.0 0.0001)
    (if (< (`self.RotationSpeed`) 0.0)
      (set `self.RotationSpeed` (+ (`self.RotationSpeed`) (* (`GameplayStatics.GetWorldDeltaSeconds`) (`self.RotationAcceleration`))))
      (else
        (set `self.RotationSpeed` (- (`self.RotationSpeed`) (* (`GameplayStatics.GetWorldDeltaSeconds`) (`self.RotationAcceleration`))))))
    (if (`KismetMathLibrary.NearlyEqual_FloatFloat` (`self.RotationSpeed`) 0.0 0.1)
      (set `self.RotationSpeed` 0.0))
    (else
      (set `self.RotationSpeed` (+ (`self.RotationSpeed`) (* AxisValue (`GameplayStatics.GetWorldDeltaSeconds`) (`self.RotationAcceleration`))))))
  (`SceneComponent.K2_AddLocalRotation` (`self.Cylinder`) (`KismetMathLibrary.MakeRotator` 0.0 0.0 (`self.RotationSpeed`)) false false))

(fn `NewFunction_0`
  (if true
    _))

(fn `UserConstructionScript`)